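; Scissors weapon that cuts and dyes hair on the wielder or other players and shears haircuttable dinos, with an option to stop hair regrowing.
; Melee montage notifies open HairStyleUINoGrow for the wielder or traced player, or request a dino haircut.
; Server events check range, line of sight and PVE team, then apply styles, grant hair, consume dye and durability.
; The growth toggle adds or removes Buff_NoHairGrowth, which receives the cut lengths.
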(event Custom|OnHairGrowthChanged_Event
  (params (HairGrowthDisabled :type Boolean))
  (Variables|Default|SetDisableHairGrowth HairGrowthDisabled))

(event Custom|DoServerRequestDinoHaircut
  (params (DoRequestOnDino :type Dino%20Character%20BP%20Haircuttable%20Object%20Reference))
  (bind _associatedprimalitem (Variables|Default|GetAssociatedPrimalItem))
  (bind _mypawn (Variables|Default|GetMyPawn))
  (Utilities|IsValid DoRequestOnDino
    (:Is%20Valid
      (Utilities|IsValid _mypawn
        (:Is%20Valid
          (bind _bisvalid (CallFunction|IsValidHairCutTarget DoRequestOnDino))
          (if _bisvalid
            (Default|DoHaircut DoRequestOnDino _mypawn)
            (Utilities|IsValid _associatedprimalitem
              (:Is%20Valid
                (Class|PrimalItem|AddItemDurability _associatedprimalitem (Variables|Default|GetOnDinoItemDurabilityToSubtract))))))))))

(event Custom|InitializeUI
  (params (TheUI :type UI%20Hairstyle%20Object%20Reference))
  (EventDispatchers|BindEventtoTheHairStyleSelectedDelegate TheUI (delegate Custom|OnHairStyleAccepted__DelegateSignature_Event))
  (EventDispatchers|BindEventtoClearFacialHairButtonClickedDelegate TheUI (delegate Custom|ClearFacialHairClicked))
  (EventDispatchers|BindEventtoClearHeadHairButtonClickedDelegate TheUI (delegate Custom|ClearHeadHairClicked))
  (bind _ashairstyleuinogrow_c (Utilities|Casting|CastToHairStyleUINoGrow TheUI))
  (EventDispatchers|BindEventtoOnHairGrowthChanged _ashairstyleuinogrow_c (delegate Custom|OnHairGrowthChanged_Event)))

(event Custom|TheServerHairStyleAccepted
  (params (NewHeadHairIndex :type Integer) (NewFacialHairIndex :type Integer) (NewHeadHairPercent :type Float%20%28single-precision%29) (NewFacialHairPercent :type Float%20%28single-precision%29) (HeadHairDyeID1 :type Integer) (HeadHairDyeID2 :type Integer) (FacialHairDyeID1 :type Integer) (FacialHairDyeID2 :type Integer) (ForTarget :type Shooter%20Character%20Object%20Reference) (DisableHairGrowth :type Boolean))
  (bind _returnvalue (Class|ShooterCharacter|GetPercentageOfFacialHairGrowth ForTarget))
  (bind _returnvalue_2 (Class|ShooterCharacter|GetPercentageOfHeadHairGrowth ForTarget))
  (bind _mypawn (Variables|Default|GetMyPawn))
  (bind _dyehaircolorsaturation (Variables|Default|GetDyeHairColorSaturation))
  (bind _myinventorycomponent (Variables|/Script/ShooterGame.PrimalCharacter|GetMyInventoryComponent _mypawn))
  (bind _bisvalid (CallFunction|IsValidHairCutTarget ForTarget))
  (if (Class|PrimalCharacter|IsAlive ForTarget)
    (Variables|Default|SetDisableHairGrowth DisableHairGrowth)
    (Class|GameState|BPNetSpawnActoratLocation (Game|GetGameState) "/Game/PrimalEarth/General/HairCutEmitter.HairCutEmitter_C" (Transformation|GetActorLocation) "0, 0, 0" 0 2e+03 0 0 "None" false)
    (if _bisvalid
      (if (Class|VictoryCore|IsShipping)
        (Variables|Default|SetbAllowPositiveHaircut false))
      (Variables|Default|SetItemDurabilityToSubtract (Math|Float|Min(Float) (+ (* (- _returnvalue_2 (Math|Float|Min(Float) (select (or (== (Class|ShooterCharacter|GetHeadHairIndex ForTarget) NewHeadHairIndex) (Variables|Default|GetbAllowPositiveHaircut)) NewHeadHairPercent 0.0) (select (Variables|Default|GetbAllowPositiveHaircut) 1.0 _returnvalue_2))) (Variables|Default|GetHeadHairCutDurabilityCostPerPercent)) (* (Variables|Default|GetFacialHairCutDurabilityCostPerPercent) (- _returnvalue (Math|Float|Min(Float) (select (or (== (Class|ShooterCharacter|GetFacialHairIndex ForTarget) NewFacialHairIndex) (Variables|Default|GetbAllowPositiveHaircut)) NewFacialHairPercent 0.0) (select (Variables|Default|GetbAllowPositiveHaircut) 1.0 _returnvalue))))) (Variables|Default|GetMinCutDurabilityCost)))
      (CallFunction|GiveHairLocks (Math|Float|Floor (* (- _returnvalue_2 (Math|Float|Min(Float) (select (or (== (Class|ShooterCharacter|GetHeadHairIndex ForTarget) NewHeadHairIndex) (Variables|Default|GetbAllowPositiveHaircut)) NewHeadHairPercent 0.0) (select (Variables|Default|GetbAllowPositiveHaircut) 1.0 _returnvalue_2))) (Variables|Default|GetHeadHairLocksPerPercent))))
      (Class|ShooterCharacter|NetSetHeadHairPercent ForTarget (Math|Float|Min(Float) (select (or (== (Class|ShooterCharacter|GetHeadHairIndex ForTarget) NewHeadHairIndex) (Variables|Default|GetbAllowPositiveHaircut)) NewHeadHairPercent 0.0) (select (Variables|Default|GetbAllowPositiveHaircut) 1.0 _returnvalue_2)) NewHeadHairIndex)
      (CallFunction|GiveHairLocks (Math|Float|Floor (* (- _returnvalue (Math|Float|Min(Float) (select (or (== (Class|ShooterCharacter|GetFacialHairIndex ForTarget) NewFacialHairIndex) (Variables|Default|GetbAllowPositiveHaircut)) NewFacialHairPercent 0.0) (select (Variables|Default|GetbAllowPositiveHaircut) 1.0 _returnvalue))) (Variables|Default|GetFacialHairLocksPerPercent))))
      (Class|ShooterCharacter|NetSetFacialHairPercent ForTarget (Math|Float|Min(Float) (select (or (== (Class|ShooterCharacter|GetFacialHairIndex ForTarget) NewFacialHairIndex) (Variables|Default|GetbAllowPositiveHaircut)) NewFacialHairPercent 0.0) (select (Variables|Default|GetbAllowPositiveHaircut) 1.0 _returnvalue)) NewFacialHairIndex)
      (Utilities|FlowControl|Sequence
        (:then_0
          (bind _returnvalue_3 (Class|PrimalInventoryComponent|BPFindItemwithID _myinventorycomponent HeadHairDyeID1 HeadHairDyeID2))
          (bind _asprimalitem_dye (Utilities|Casting|CastToPrimalItem_Dye _returnvalue_3))
          (Class|ShooterCharacter|NetSetOverrideHeadHairColor ForTarget (Class|VictoryCore|ChangeSaturation (Variables|/Script/ShooterGame.PrimalItem_Dye|GetDyeColor _asprimalitem_dye) _dyehaircolorsaturation))
          (bind _asprimalitem (Utilities|Casting|CastToPrimalItemClass (Utilities|GetClass _asprimalitem_dye)))
          (Class|PrimalInventoryComponent|BPIncrementItemTemplateQuantity _myinventorycomponent _asprimalitem -1 true false true false true false _asprimalitem_dye false))
        (:then_1
          (bind _returnvalue_4 (Class|PrimalInventoryComponent|BPFindItemwithID _myinventorycomponent FacialHairDyeID1 FacialHairDyeID2))
          (bind _asprimalitem_dye_2 (Utilities|Casting|CastToPrimalItem_Dye _returnvalue_4))
          (Class|ShooterCharacter|NetSetOverrideFacialHairColor ForTarget (Class|VictoryCore|ChangeSaturation (Variables|/Script/ShooterGame.PrimalItem_Dye|GetDyeColor _asprimalitem_dye_2) _dyehaircolorsaturation))
          (bind _asprimalitem_2 (Utilities|Casting|CastToPrimalItemClass (Utilities|GetClass _asprimalitem_dye_2)))
          (Class|PrimalInventoryComponent|BPIncrementItemTemplateQuantity _myinventorycomponent _asprimalitem_2 -1 true false true false true false _asprimalitem_dye_2 false))
        (:then_2
          (if (< (Variables|Default|GetItemDurabilityToSubtract) 0.0)
            (Class|PrimalItem|AddItemDurability (Variables|Default|GetAssociatedPrimalItem) (Variables|Default|GetItemDurabilityToSubtract))))
        (:then_3
          (if (Variables|Default|GetDisableHairGrowth)
            (bind _returnvalue_5 (Class|PrimalCharacter|HasBuff ForTarget "/Game/Mods/GenericMod/NoHairGrowScissors/Buffs/Buff_NoHairGrowth.Buff_NoHairGrowth_C" false))
            (if _returnvalue_5
              (bind _returnvalue_6 (Class|PrimalCharacter|GetBuff ForTarget "/Game/Mods/GenericMod/NoHairGrowScissors/Buffs/Buff_NoHairGrowth.Buff_NoHairGrowth_C"))
              (bind _asbuff_nohairgrowth_c (Utilities|Casting|CastToBuff_NoHairGrowth _returnvalue_6))
              (Default|InitBuff _asbuff_nohairgrowth_c NewHeadHairIndex (Math|Float|Min(Float) (select (or (== (Class|ShooterCharacter|GetHeadHairIndex ForTarget) NewHeadHairIndex) (Variables|Default|GetbAllowPositiveHaircut)) NewHeadHairPercent 0.0) (select (Variables|Default|GetbAllowPositiveHaircut) 1.0 _returnvalue_2)) NewFacialHairIndex (Math|Float|Min(Float) (select (or (== (Class|ShooterCharacter|GetFacialHairIndex ForTarget) NewFacialHairIndex) (Variables|Default|GetbAllowPositiveHaircut)) NewFacialHairPercent 0.0) (select (Variables|Default|GetbAllowPositiveHaircut) 1.0 _returnvalue)))
              (else
                (bind _returnvalue_7 (Class|PrimalBuff|StaticAddBuff "/Game/Mods/GenericMod/NoHairGrowScissors/Buffs/Buff_NoHairGrowth.Buff_NoHairGrowth_C" ForTarget 0 0 true))
                (bind _asbuff_nohairgrowth_c_2 (Utilities|Casting|CastToBuff_NoHairGrowth _returnvalue_7))
                (Default|InitBuff _asbuff_nohairgrowth_c_2 NewHeadHairIndex (Math|Float|Min(Float) (select (or (== (Class|ShooterCharacter|GetHeadHairIndex ForTarget) NewHeadHairIndex) (Variables|Default|GetbAllowPositiveHaircut)) NewHeadHairPercent 0.0) (select (Variables|Default|GetbAllowPositiveHaircut) 1.0 _returnvalue_2)) NewFacialHairIndex (Math|Float|Min(Float) (select (or (== (Class|ShooterCharacter|GetFacialHairIndex ForTarget) NewFacialHairIndex) (Variables|Default|GetbAllowPositiveHaircut)) NewFacialHairPercent 0.0) (select (Variables|Default|GetbAllowPositiveHaircut) 1.0 _returnvalue)))))
            (else
              (bind _returnvalue_8 (Class|PrimalCharacter|HasBuff ForTarget "/Game/Mods/GenericMod/NoHairGrowScissors/Buffs/Buff_NoHairGrowth.Buff_NoHairGrowth_C" false))
              (if _returnvalue_8
                (Class|PrimalCharacter|DeactivateBuffs ForTarget "/Game/Mods/GenericMod/NoHairGrowScissors/Buffs/Buff_NoHairGrowth.Buff_NoHairGrowth_C" 0 false)))))))))

(event Custom|ClearFacialHairClicked
  (CallFunction|ServerClearFacialHairColor (Variables|Default|GetHairCutTarget)))

(event Custom|ClearHeadHairClicked
  (CallFunction|ServerClearHeadHairColor (Variables|Default|GetHairCutTarget)))

(event Custom|ServerClearFacialHairColor
  (params (TargetChar :type Shooter%20Character%20Object%20Reference))
  (bind _bisvalid (CallFunction|IsValidHairCutTarget TargetChar))
  (if _bisvalid
    (Class|ShooterCharacter|NetSetOverrideFacialHairColor TargetChar (Variables|/Script/ShooterGame.ShooterCharacter|GetOriginalHairColor TargetChar))))

(event Custom|ServerClearHeadHairColor
  (params (TargetChar :type Shooter%20Character%20Object%20Reference))
  (bind _bisvalid (CallFunction|IsValidHairCutTarget TargetChar))
  (if _bisvalid
    (Class|ShooterCharacter|NetSetOverrideHeadHairColor TargetChar (Variables|/Script/ShooterGame.ShooterCharacter|GetOriginalHairColor TargetChar))))

(event Custom|OnHairStyleAccepted__DelegateSignature_Event
  (params (NewHeadHairIndex :type Integer) (NewFacialHairIndex :type Integer) (NewHeadHairPercent :type Float%20%28single-precision%29) (NewFacialHairPercent :type Float%20%28single-precision%29) (HeadHairDyeID1 :type Integer) (HeadHairDyeID2 :type Integer) (FacialHairDyeID1 :type Integer) (FacialHairDyeID2 :type Integer))
  (CallFunction|TheServerHairStyleAccepted NewHeadHairIndex NewFacialHairIndex NewHeadHairPercent NewFacialHairPercent HeadHairDyeID1 HeadHairDyeID2 FacialHairDyeID1 FacialHairDyeID2 (Variables|Default|GetHairCutTarget) (Variables|Default|GetDisableHairGrowth)))

(fn ConstructionScript)

(fn BPGetSelectedMeleeAttackAnim
  (bind _bwantstofire (Variables|Default|GetbWantsToFire))
  (bind _returnvalue (not _bwantstofire))
  (return (Utilities|Struct|MakeWeaponAnim (select _returnvalue "/Game/PrimalEarth/WeaponScissors/Animations/FPV/FPV_Scissors_WP_Haircut_Montage.FPV_Scissors_WP_Haircut_Montage" "/Game/PrimalEarth/WeaponScissors/Animations/FPV/FPV_Scissors_WP_Attack_Montage.FPV_Scissors_WP_Attack_Montage") (select _returnvalue "/Game/PrimalEarth/WeaponScissors/Animations/TPV/TPV_Scissors_HM_Attack_Montage_Slower.TPV_Scissors_HM_Attack_Montage_Slower" "/Game/PrimalEarth/WeaponScissors/Animations/TPV/TPV_Scissors_HM_Attack_Montage.TPV_Scissors_HM_Attack_Montage"))))

(fn BPAnimNotifyCustomEvent
  (params (CustomEventName :type Name :default "None") (MeshComp :type Skeletal%20Mesh%20Component%20Object%20Reference) (Animation :type Anim%20Sequence%20Base%20Object%20Reference) (AnimNotifyObject :type Anim%20Notify%20Object%20Reference))
  (bind _mypawn (Variables|Default|GetMyPawn))
  (bind _returnvalue (Pawn|GetController _mypawn))
  (bind (_location _rotation) (Pawn|GetPlayerViewPoint _returnvalue))
  (if (and (Pawn|IsLocallyControlled _mypawn) (Utilities|IsValid _returnvalue))
    (switch name CustomEventName
      (:CutHead
        (CallFunction|OpenUI _mypawn))
      (:CutFacial
        (bind (_outhit _returnvalue_2) (Collision|LineTraceByChannel _location (+ _location (* (Math|Vector|GetForwardVector _rotation) 1.6e+02)) "ECC_GameTraceChannel1" true (Utilities|Array|MakeArray _mypawn) "None"))
        (if _returnvalue_2
          (bind _asshootercharacter (Utilities|Casting|CastToShooterCharacter (.HitActor (Collision|BreakHitResult _outhit)))
            (:then
              (bind _bisvalid (CallFunction|IsValidHairCutTarget _asshootercharacter))
              (if _bisvalid
                (if (Class|PrimalCharacter|IsAlive _asshootercharacter)
                  (CallFunction|OpenUI _asshootercharacter))))
            (:CastFailed
              (bind _asdino_character_bp_haircuttable_c (Utilities|Casting|CastToDino_Character_BP_Haircuttable (.HitActor (Collision|BreakHitResult _outhit))))
              (CallFunction|DoServerRequestDinoHaircut _asdino_character_bp_haircuttable_c))))))))

(fn GiveHairLocks
  (params (NumLocks :type Integer))
  (bind _mypawn (Variables|Default|GetMyPawn))
  (bind _myinventorycomponent (Variables|/Script/ShooterGame.PrimalCharacter|GetMyInventoryComponent _mypawn))
  (if (> NumLocks 0)
    (Utilities|IsValid _mypawn
      (:Is%20Valid
        (Utilities|IsValid _myinventorycomponent
          (:Is%20Valid
            (Class|PrimalItem|AddNewItem "/Game/PrimalEarth/CoreBlueprints/Resources/PrimalItemResource_Hair.PrimalItemResource_Hair_C" _myinventorycomponent false false 0.0 true NumLocks false 0.0 false 0 0.0)))))))

(fn OpenUI
  (params (TheTarget :type Shooter%20Character%20Object%20Reference))
  (Variables|Default|SetHairCutTarget TheTarget)
  (bind _asshooterplayercontroller (Utilities|Casting|CastToShooterPlayerController (Pawn|GetController (Variables|Default|GetMyPawn))))
  (bind _asshooterhud (Utilities|Casting|CastToShooterHUD (HUD|GetHUD _asshooterplayercontroller)))
  (bind _returnvalue (Class|ShooterHUD|BPShowUIScene _asshooterhud "/Game/Mods/GenericMod/NoHairGrowScissors/UI/HairStyleUINoGrow.HairStyleUINoGrow_C" (Variables|Default|GetHairCutTarget) 0 (Math|Conversions|ToInteger(Boolean) (Variables|Default|GetbAllowPositiveHaircut)) (Math|Float|Ceil (* (Variables|Default|GetDyeHairColorSaturation) 1e+03))))
  (bind _ashairstyleuinogrow_c (Utilities|Casting|CastToHairStyleUINoGrow _returnvalue))
  (CallFunction|InitializeUI _ashairstyleuinogrow_c))

(fn IsValidHairCutTarget
  (params (PotentialTarget :type Actor%20Object%20Reference))
  (bind _returnvalue (Transformation|GetActorLocation PotentialTarget))
  (bind _mypawn (Variables|Default|GetMyPawn))
  (bind _returnvalue_2 (Pawn|GetController _mypawn))
  (LocalVariables|SetretVal false)
  (Utilities|FlowControl|Sequence
    (:then_0
      (Utilities|IsValid PotentialTarget
        (:Is%20Valid
          (Utilities|IsValid _mypawn
            (:Is%20Valid
              (Utilities|IsValid _returnvalue_2
                (:Is%20Valid
                  (Utilities|IsValid (Variables|Default|GetAssociatedPrimalItem)
                    (:Is%20Valid
                      (bind _asshootergamestate (Utilities|Casting|CastToShooterGameState (Game|GetGameState)))
                      (if (Math|Boolean|ORBoolean (not (Variables|/Script/ShooterGame.ShooterGameState|GetbServerPVE _asshootergamestate)) (== (Variables|/Script/Engine.Actor|GetTargetingTeam _mypawn) (Variables|/Script/Engine.Actor|GetTargetingTeam PotentialTarget)) (Class|Actor|IsPrimalDino PotentialTarget))
                        (if (< (Math|Vector|VectorLength (- _returnvalue (Transformation|GetActorLocation _mypawn))) 3.3e+02)
                          (bind _returnvalue_3 (Collision|LineTraceByChannel (.Location (Pawn|GetPlayerViewPoint _returnvalue_2)) _returnvalue "ECC_GameTraceChannel11" true 0 "None"))
                          (LocalVariables|SetretVal (not _returnvalue_3)))))))))))))
    (:then_1
      (return (LocalVariables|GetretVal)))))

(fn ReceiveBeginPlay
  (if (Class|VictoryCore|IsShipping)
    (Variables|Default|SetbAllowPositiveHaircut false)))